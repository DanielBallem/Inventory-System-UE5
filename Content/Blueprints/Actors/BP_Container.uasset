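; BP_Container is a world container actor with its own inventory that can be shown alongside a player's inventory.
; BeginPlay seeds its inventory component with hardcoded wood and armor pieces, creates a WBP_Inventory bound to that component, and hands the widget back before calling SetUIEvent.
; OpenContainer creates a WBP_ContainerAccess from the passed player inventory and the container's prebuilt inventory widget, then adds it to the viewport.
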(event EventBeginPlay
  (bind _myinventorycomponent (Variables|Default|GetMyInventoryComponent))
  (bind _myinventorycomponent_2 (Variables|Default|GetMyInventoryComponent))
  (Class|InventoryComponent|DropItemIntoInventory _myinventorycomponent_2 "Wood" 5)
  (Class|InventoryComponent|DropItemIntoInventory _myinventorycomponent_2 "DHelm" 2)
  (Class|InventoryComponent|DropItemIntoInventory _myinventorycomponent_2 "DChest" 2)
  (Class|InventoryComponent|DropItemIntoInventory _myinventorycomponent_2 "DLegs" 2)
  (Class|InventoryComponent|DropItemIntoInventory _myinventorycomponent_2 "DBoots" 2)
  (bind _returnvalue (UserInterface|CreateWidget "/Game/Widgets/Inventory/WBP_Inventory.WBP_Inventory_C" 0 _myinventorycomponent))
  (bind _output_get (Variables|Default|SetInventoryWidget _returnvalue))
  (Variables|/Game/Blueprints/Components/BP_InventoryComponent.BP_InventoryComponent_C|SetinventoryWidget _myinventorycomponent _output_get)
  (Default|SetUIEvent _myinventorycomponent))

(event Collision|EventActorBeginOverlap
  (params (OtherActor :type Actor%20Object%20Reference)))

(event EventTick
  (params (DeltaSeconds :type Float%20%28single-precision%29)))

(fn ConstructionScript)

(fn OpenContainer
  (params (PlayerInventory :type WBP%20Inventory%20Object%20Reference))
  (bind _returnvalue (UserInterface|CreateWidget "/Game/Widgets/Inventory/WBP_ContainerAccess.WBP_ContainerAccess_C" 0 PlayerInventory (Variables|Default|GetInventoryWidget)))
  (UserInterface|Viewport|AddtoViewport _returnvalue 0)
  (return))