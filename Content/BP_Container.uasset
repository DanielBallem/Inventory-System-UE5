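; BP_Container is a world container actor with its own inventory component, pre-stocked with Wood on BeginPlay.
; On BeginPlay it creates a WBP_Inventory widget bound to that component, hands the widget back to the component and calls SetUIEvent.
; OpenContainer takes the player's inventory and shows a WBP_ContainerAccess widget that pairs it with the container's inventory widget.
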(event EventBeginPlay
  (bind _myinventorycomponent (Variables|Default|GetMyInventoryComponent))
  (Class|InventoryComponent|DropItemIntoInventory (Variables|Default|GetMyInventoryComponent) "Wood" 5)
  (bind _returnvalue (UserInterface|CreateWidget "/Game/WBP_Inventory.WBP_Inventory_C" 0 _myinventorycomponent))
  (bind _output_get (Variables|Default|SetInventoryWidget _returnvalue))
  (Variables|/Game/MyInventoryComponent.MyInventoryComponent_C|SetinventoryWidget _myinventorycomponent _output_get)
  (Default|SetUIEvent _myinventorycomponent))

(event Collision|EventActorBeginOverlap
  (params (OtherActor :type Actor%20Object%20Reference)))

(event EventTick
  (params (DeltaSeconds :type Float%20%28single-precision%29)))

(fn ConstructionScript)

(fn OpenContainer
  (params (PlayerInventory :type WBP%20Inventory%20Object%20Reference))
  (bind _returnvalue (UserInterface|CreateWidget "/Game/WBP_ContainerAccess.WBP_ContainerAccess_C" 0 PlayerInventory (Variables|Default|GetInventoryWidget)))
  (UserInterface|Viewport|AddtoViewport _returnvalue 0)
  (return))